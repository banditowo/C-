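; BP_Projectile is a short-lived projectile actor that credits players for dodging it.
; It destroys itself after a fixed delay from BeginPlay.
; A hit on the Cone component sets the HitCone flag.
; While that flag is unset, each overlap of the Collide component with a BP_MyPlayers actor increments that player's Dodged count.
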(event OnComponentHit(Cone)
  (params (HitComponent :type Primitive%20Component%20Object%20Reference) (OtherActor :type Actor%20Object%20Reference) (OtherComp :type Primitive%20Component%20Object%20Reference) (NormalImpulse :type Vector :default "0, 0, 0") (Hit :type Hit%20Result%20Structure%20%28by%20ref%29))
  (Variables|Default|SetHitCone true))

(event OnComponentBeginOverlap(Collide)
  (params (OverlappedComponent :type Primitive%20Component%20Object%20Reference) (OtherActor :type Actor%20Object%20Reference) (OtherComp :type Primitive%20Component%20Object%20Reference) (OtherBodyIndex :type Integer) (bFromSweep :type Boolean) (SweepResult :type Hit%20Result%20Structure%20%28by%20ref%29))
  (if (not (Variables|Default|GetHitCone))
    (bind _asbp_my_players (Utilities|Casting|CastToBP_MyPlayers OtherActor))
    (Variables|/Game/Blueprints/BP_MyPlayers.BP_MyPlayers_C|SetDodged _asbp_my_players (+ 1 (Variables|/Game/Blueprints/BP_MyPlayers.BP_MyPlayers_C|GetDodged _asbp_my_players)))))

(event EventBeginPlay
  (Utilities|FlowControl|Delay 5.0)
  (Actor|DestroyActor))

(event Collision|EventActorBeginOverlap
  (params (OtherActor :type Actor%20Object%20Reference)))

(event EventTick
  (params (DeltaSeconds :type Float%20%28single-precision%29)))

(fn ConstructionScript)