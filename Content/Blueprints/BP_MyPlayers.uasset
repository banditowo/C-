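; Single pawn that runs a two-player endless runner, holding both player components, a shared auto-scrolling camera and the score and lives widgets.
; Tick advances camera and players, copies EndlessRunnerScoreSystem's score to living players and reloads the level once both die.
; Pipe hits cost lives and trigger timer-driven flicker invincibility, while "CanKill" overlaps kill outright.
; Enhanced Input moves each player, and a looping timer randomly spawns projectiles.
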(event OnComponentBeginOverlap(Player1)
  (params (OverlappedComponent :type Primitive%20Component%20Object%20Reference) (OtherActor :type Actor%20Object%20Reference) (OtherComp :type Primitive%20Component%20Object%20Reference) (OtherBodyIndex :type Integer) (bFromSweep :type Boolean) (SweepResult :type Hit%20Result%20Structure%20%28by%20ref%29))
  ;[1 1 1] KillBox
  (if (Components|ComponentHasTag OtherComp "CanKill")
    (Variables|Default|SetPlayer1Lives 0)
    (CallFunction|KillP1)))

(event OnComponentBeginOverlap(Player2)
  (params (OverlappedComponent :type Primitive%20Component%20Object%20Reference) (OtherActor :type Actor%20Object%20Reference) (OtherComp :type Primitive%20Component%20Object%20Reference) (OtherBodyIndex :type Integer) (bFromSweep :type Boolean) (SweepResult :type Hit%20Result%20Structure%20%28by%20ref%29))
  ;[1 1 1] KillBox
  (if (Components|ComponentHasTag OtherComp "CanKill")
    (Variables|Default|SetPlayer2Lives 0)
    (CallFunction|KillP2)))

(event OnComponentHit(Player1)
  (params (HitComponent :type Primitive%20Component%20Object%20Reference) (OtherActor :type Actor%20Object%20Reference) (OtherComp :type Primitive%20Component%20Object%20Reference) (NormalImpulse :type Vector :default "0, 0, 0") (Hit :type Hit%20Result%20Structure%20%28by%20ref%29))
  ;[1 1 1] Player Lives
  (Utilities|Casting|CastToBP_Pipes OtherActor)
  (Variables|Default|Setplayer1Invincible true)
  (CallFunction|P1Incinvibility)
  (Variables|Default|SetPlayer1Lives (- (Variables|Default|GetPlayer1Lives) 1))
  (CallFunction|KillP1))

(event OnComponentHit(Player2)
  (params (HitComponent :type Primitive%20Component%20Object%20Reference) (OtherActor :type Actor%20Object%20Reference) (OtherComp :type Primitive%20Component%20Object%20Reference) (NormalImpulse :type Vector :default "0, 0, 0") (Hit :type Hit%20Result%20Structure%20%28by%20ref%29))
  ;[1 1 1] Player Lives
  (Utilities|Casting|CastToBP_Pipes OtherActor)
  (Variables|Default|Setplayer2Invincible true)
  (CallFunction|P2Invincibility)
  (Variables|Default|SetPlayer2Lives (- (Variables|Default|GetPlayer2Lives) 1))
  (CallFunction|KillP2))

(event Custom|SpawnProjectiles
  ;[1 1 1] BeginPlay
  (switch int (Math|Random|RandomIntegerinRange 0 2)
    (:0
      (if (not (and (> (Variables|Default|GetDodged) 0) (== (Math|Random|RandomIntegerinRange 0 10) 10)))
        (Game|SpawnActorfromClass "/Game/Blueprints/BP_Projectile.BP_Projectile_C" (Transformation|GetWorldTransform (Variables|Default|GetProjectileSpawner)) "Undefined" 0 0)
        (Variables|Default|SetDodged (- (Variables|Default|GetDodged) 1))))))

(event Custom|ResetLevel
  ;[1 1 1] Reset Level
  (if (and (Variables|Default|Getplayer1Dead) (Variables|Default|Getplayer2Dead))
    (Utilities|FlowControl|Delay 0.5)
    (bind _returnvalue (Game|GetCurrentLevelName true))
    (Game|OpenLevel(byName) (Utilities|String|StringToName _returnvalue))))

(event Custom|FlickerP2
  ;[1 1 1] Player Invincibility
  (Rendering|ToggleVisibility (Variables|Default|GetPlayer2) false))

(event Custom|FlickerP1
  ;[1 1 1] Player Invincibility
  (Rendering|ToggleVisibility (Variables|Default|GetPlayer1) false))

(event Custom|P2Invincibility
  (bind _player2 (Variables|Default|GetPlayer2))
  (bind _player2_2 (Variables|Default|GetPlayer2))
  ;[1 1 1] Player Invincibility
  (if (and (Variables|Default|Getplayer2Invincible) (> (Variables|Default|GetPlayer2Lives) 1))
    (Physics|SetSimulatePhysics _player2 false)
    (Collision|SetCollisionEnabled _player2 "QueryOnly")
    (bind _returnvalue (Utilities|Time|SetTimerbyEvent (delegate Custom|FlickerP2) 0.1 true))
    (bind _output_get (Variables|Default|SetNewVar _returnvalue))
    (Utilities|FlowControl|Delay 1.0)
    (Utilities|Time|ClearandInvalidateTimerbyHandle _output_get)
    (Rendering|SetVisibility _player2_2 true false)
    (Physics|SetSimulatePhysics (Variables|Default|GetPlayer2) true)
    (Collision|SetCollisionEnabled _player2_2 "QueryAndPhysics")
    (Variables|Default|Setplayer2Invincible false)))

(event Custom|P1Incinvibility
  (bind _player1 (Variables|Default|GetPlayer1))
  (bind _player1_2 (Variables|Default|GetPlayer1))
  ;[1 1 1] Player Invincibility
  (if (and (Variables|Default|Getplayer1Invincible) (> (Variables|Default|GetPlayer1Lives) 1))
    (Physics|SetSimulatePhysics _player1 false)
    (Collision|SetCollisionEnabled _player1 "QueryOnly")
    (bind _returnvalue (Utilities|Time|SetTimerbyEvent (delegate Custom|FlickerP1) 0.1 true))
    (bind _output_get (Variables|Default|SetNewVar _returnvalue))
    (Utilities|FlowControl|Delay 1.0)
    (Utilities|Time|ClearandInvalidateTimerbyHandle _output_get)
    (Rendering|SetVisibility _player1_2 true false)
    (Physics|SetSimulatePhysics (Variables|Default|GetPlayer1) true)
    (Collision|SetCollisionEnabled _player1_2 "QueryAndPhysics")
    (Variables|Default|Setplayer1Invincible false)))

(event Input|EnhancedActionEvents|EnhancedInputActionP1Move_IA
  (params (ActionValue :type Vector :default "0, 0, 0") (ElapsedSeconds :type Float%20%28double-precision%29) (TriggeredSeconds :type Float%20%28double-precision%29) (InputAction :type Input%20Action%20Object%20Reference :default "/Game/Input/P1Move_IA.P1Move_IA"))
  ;[1 1 1] Player Inputs
  (:Triggered
    (Utilities|IsValid (Variables|Default|GetPlayer1)
      (:Is%20Valid
        (if (not (Variables|Default|Getplayer1Dead))
          (Transformation|AddRelativeLocation (Variables|Default|GetPlayer1) (Math|Vector|MakeVector 0.0 (* (.y ActionValue) (Variables|Default|GetFaster)) (* (.x ActionValue) (Variables|Default|GetSpeed))) false false))))))

(event Input|EnhancedActionEvents|EnhancedInputActionP2Move_IA
  (params (ActionValue :type Vector :default "0, 0, 0") (ElapsedSeconds :type Float%20%28double-precision%29) (TriggeredSeconds :type Float%20%28double-precision%29) (InputAction :type Input%20Action%20Object%20Reference :default "/Game/Input/P2Move_IA.P2Move_IA"))
  ;[1 1 1] Player Inputs
  (:Triggered
    (Utilities|IsValid (Variables|Default|GetPlayer2)
      (:Is%20Valid
        (if (not (Variables|Default|Getplayer2Dead))
          (Transformation|AddRelativeLocation (Variables|Default|GetPlayer2) (Math|Vector|MakeVector 0.0 (* (.y ActionValue) (Variables|Default|GetFaster)) (* (.x ActionValue) (Variables|Default|GetSpeed))) false false))))))

(event EventTick
  (params (DeltaSeconds :type Float%20%28single-precision%29))
  (bind _player2 (Variables|Default|GetPlayer2))
  (bind _player1 (Variables|Default|GetPlayer1))
  (bind _slower (Variables|Default|GetSlower))
  ;[1 1 1] Event Tick/Player Movement
  (Utilities|FlowControl|Sequence
    (:then_0
      (Transformation|AddRelativeLocation (Variables|Default|GetCamera) (Math|Vector|MakeVector 0.0 (Variables|Default|GetSpeed) 0.0) false false))
    (:then_1
      (Utilities|IsValid _player2
        (:Is%20Valid
          (if (not (Variables|Default|Getplayer2Dead))
            (Transformation|AddRelativeLocation _player2 (Math|Vector|MakeVector 0.0 _slower 0.0) false false)))))
    (:then_2
      (CallFunction|ResetLevel))
    (:then_3
      (Utilities|IsValid _player1
        (:Is%20Valid
          (if (not (Variables|Default|Getplayer1Dead))
            (Transformation|AddRelativeLocation _player1 (Math|Vector|MakeVector 0.0 _slower 0.0) false false)))))
    (:then_4
      (CallFunction|UpdateScore))))

(event EventBeginPlay
  ;[1 1 1] BeginPlay
  (Utilities|FlowControl|Sequence
    (:then_0
      (CallFunction|ScoreWidgetF))
    (:then_1
      (CallFunction|LivesWidgetF))
    (:then_2
      (CallFunction|EnhancedInput))
    (:then_3
      (CallFunction|SetSpeeds))
    (:then_4
      (Variables|Default|Setplayer1Dead false)
      (Variables|Default|Setplayer2Dead false)
      (CallFunction|ResetLevel))
    (:then_5
      (bind _returnvalue (Actor|GetActorOfClass "/Script/EndlessRunner.EndlessRunnerScoreSystem"))
      (Variables|Default|SetScoreSystem _returnvalue))
    (:then_6
      (Utilities|Time|SetTimerbyEvent (delegate Custom|SpawnProjectiles) (Math|Random|RandomFloatinRange 0.5 2.5) true))))

(fn ConstructionScript)

(fn KillP1
  (if (== (Variables|Default|GetPlayer1Lives) 0)
    (Variables|Default|Setplayer1Dead true)
    (Components|DestroyComponent (Variables|Default|GetPlayer1))))

(fn KillP2
  (if (== (Variables|Default|GetPlayer2Lives) 0)
    (Variables|Default|Setplayer2Dead true)
    (Components|DestroyComponent (Variables|Default|GetPlayer2))))

(fn ScoreWidgetF
  (bind _returnvalue (UserInterface|CreateWidget "/Game/Blueprints/WBP_Score.WBP_Score_C"))
  (bind _output_get (Variables|Default|SetScoreWidget _returnvalue))
  (UserInterface|Viewport|AddtoViewport _output_get 0))

(fn LivesWidgetF
  (bind _returnvalue (UserInterface|CreateWidget "/Game/Blueprints/WBP_Lives.WBP_Lives_C"))
  (bind _output_get (Variables|Default|SetLivesWidget _returnvalue))
  (UserInterface|Viewport|AddtoViewport _output_get 0))

(fn EnhancedInput
  (bind _asplayer_controller (Utilities|Casting|CastToPlayerController (Pawn|GetController)))
  (Utilities|IsValid (PlayerController|LocalPlayerSubsystems|GetEnhancedInputLocalPlayerSubsystem _asplayer_controller)
    (:Is%20Valid
      (Input|AddMappingContext (PlayerController|LocalPlayerSubsystems|GetEnhancedInputLocalPlayerSubsystem _asplayer_controller) "/Game/Input/PlayerInput_IMC.PlayerInput_IMC" 0 "(bIgnoreAllPressedKeysUntilRelease=True,bForceImmediately=False)"))))

(fn SetSpeeds
  (bind _speed (Variables|Default|GetSpeed))
  (Variables|Default|SetFaster (* _speed 2.0))
  (Variables|Default|SetSlower (/ _speed 2.0)))

(fn UpdateScore
  (bind _scoresystem (Variables|Default|GetScoreSystem))
  (bind _returnvalue (Class|EndlessRunnerScoreSystem|GetScore _scoresystem))
  (Utilities|FlowControl|Sequence
    (:then_0
      (if (not (Variables|Default|Getplayer1Dead))
        (Variables|Default|SetPlayer1Score _returnvalue)))
    (:then_1
      (if (not (Variables|Default|Getplayer2Dead))
        (Variables|Default|SetPlayer2Score _returnvalue)))))