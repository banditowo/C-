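; BP_Pipes is a level segment that spawns the next segment as the player moves through it, forming an endless chain of pipes.
; When BP_MyPlayers first overlaps the Box trigger, a DoOnce gate lets it spawn a random class from the PipeLevels array at the ArrowEnd transform.
; The segment then destroys itself after a fixed delay, clearing the track behind the player.
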(event OnComponentBeginOverlap(Box)
  (params (OverlappedComponent :type Primitive%20Component%20Object%20Reference) (OtherActor :type Actor%20Object%20Reference) (OtherComp :type Primitive%20Component%20Object%20Reference) (OtherBodyIndex :type Integer) (bFromSweep :type Boolean) (SweepResult :type Hit%20Result%20Structure%20%28by%20ref%29))
  (bind _pipelevels (Variables|Default|GetPipeLevels))
  (Utilities|Casting|CastToBP_MyPlayers OtherActor)
  (Utilities|FlowControl|DoOnce false
    (:Completed
      (Game|SpawnActorfromClass (Utilities|Array|Get(acopy) _pipelevels (Math|Random|RandomIntegerinRange 0 (Utilities|Array|LastIndex _pipelevels))) (Transformation|GetWorldTransform (Variables|Default|GetArrowEnd)) "Undefined" 0 0)
      (Utilities|FlowControl|Delay 15.0)
      (Actor|DestroyActor))))

(fn ConstructionScript)